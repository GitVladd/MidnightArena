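; Player controller for Midnight Arena characters that binds number keys to random drains of health, mana and stamina, apparently for testing.
; Key 1 applies generic damage to every MidnightArenaCharacter in the level, while keys 2 and 3 consume from each one's ManaComponent and StaminaComponent.
; Each press gathers characters with GetAllActorsOfClass and rolls a separate random amount below a fixed cap for each.
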(event `Key|One`
  (params (Key :type "Key Structure"))
  (:`Pressed`
    (bind _outactors (`GameplayStatics.GetAllActorsOfClass` "/Script/MidnightArena.MidnightArenaCharacter"))
    (for _array_element _outactors
      (`GameplayStatics.ApplyDamage` _array_element (`KismetMathLibrary.Conv_IntToDouble` (`KismetMathLibrary.RandomInteger` 50)) null null "/Script/Engine.DamageType"))))

(event `Key|Two`
  (params (Key :type "Key Structure"))
  (:`Pressed`
    (bind _outactors (`GameplayStatics.GetAllActorsOfClass` "/Script/MidnightArena.MidnightArenaCharacter"))
    (for _array_element _outactors
      (`ManaComponent.ConsumeMana` (`BaseCharacter.ManaComponent` _array_element) (`KismetMathLibrary.Conv_IntToDouble` (`KismetMathLibrary.RandomInteger` 50))))))

(event `Key|Three`
  (params (Key :type "Key Structure"))
  (:`Pressed`
    (bind _outactors (`GameplayStatics.GetAllActorsOfClass` "/Script/MidnightArena.MidnightArenaCharacter"))
    (for _array_element _outactors
      (`StaminaComponent.ConsumeStamina` (`BaseCharacter.StaminaComponent` _array_element) (`KismetMathLibrary.Conv_IntToDouble` (`KismetMathLibrary.RandomInteger` 50))))))

(fn `UserConstructionScript`)